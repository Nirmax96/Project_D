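; BP_CineCamera_Manager is a rail camera that follows the player along a spline and serves as the player's view.
; On BeginPlay it sets itself as player controller 0's view target.
; Each Tick it snaps the Camera component to the spline point closest to the player character, without interpolation.
; It then rotates the camera to look directly at the character.
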(event EventTick
  (params (DeltaSeconds :type Float%20%28single-precision%29))
  (bind _returnvalue (Game|GetPlayerCharacter 0))
  (bind _camera (Variables|Default|GetCamera))
  (bind _returnvalue_2 (Transformation|GetActorLocation _returnvalue))
  (Transformation|SetWorldLocation _camera (Spline|FindLocationClosesttoWorldLocation (Variables|Default|GetSpline) _returnvalue_2 "World") false false)
  (Transformation|SetWorldRotation _camera (Math|Rotator|FindLookatRotation (Transformation|GetWorldLocation _camera) _returnvalue_2) false false))

(event EventBeginPlay
  (Game|Player|SetViewTargetwithBlend (Game|GetPlayerController 0) self 0.0 "VTBlend_Linear" 0.0 false))

(fn ConstructionScript)