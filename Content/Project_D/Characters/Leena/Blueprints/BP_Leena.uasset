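; Leena is a playable brawler character with camera-relative movement from a cine camera manager, melee combat against BP_Oni and ledge hanging.
; Quick and launch combos share a combo index and, like standing or running power attacks, pair montages with forward launch impulses.
; Toggled hand hitboxes damage each enemy once per activation, shaking the camera on heavier hits.
; Lock-on turns jump into a four-way dash, while per-tick traces snap Leena onto Ledge-tagged geometry.
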(event OnComponentBeginOverlap(Hitbox_LeftHand)
  (params (OverlappedComponent :type Primitive%20Component%20Object%20Reference) (OtherActor :type Actor%20Object%20Reference) (OtherComp :type Primitive%20Component%20Object%20Reference) (OtherBodyIndex :type Integer) (bFromSweep :type Boolean) (SweepResult :type Hit%20Result%20Structure%20%28by%20ref%29))
  ;[0.02423 0 1] Hit_box (test)
  (bind _asbp_oni (Utilities|Casting|CastToBP_Oni OtherActor))
  (CallFunction|DealDamagetoEnemy _asbp_oni))

(event OnComponentBeginOverlap(Hitbox_RightHand)
  (params (OverlappedComponent :type Primitive%20Component%20Object%20Reference) (OtherActor :type Actor%20Object%20Reference) (OtherComp :type Primitive%20Component%20Object%20Reference) (OtherBodyIndex :type Integer) (bFromSweep :type Boolean) (SweepResult :type Hit%20Result%20Structure%20%28by%20ref%29))
  ;[0.02423 0 1] Hit_box (test)
  (bind _asbp_oni (Utilities|Casting|CastToBP_Oni OtherActor))
  (CallFunction|DealDamagetoEnemy _asbp_oni))

(event Custom|QuickAttackImpulse
  ;[0.1651 0.08022 0.1221] Impulse_System Quick Attack
  (Pawn|Components|CharacterMovement|SetMovementMode (Variables|Character|GetCharacterMovement) "MOVE_Falling" 0)
  (Character|LaunchCharacter (* (Transformation|GetActorForwardVector) (Utilities|Select :Index (Variables|Default|GetComboIndex) :Option%200 9e+02 :Option%201 1.25e+03 :Option%202 5e+02)) true false))

(event Custom|LaunchAttackImpulse
  ;[0.01096 0.1329 0.0319] sistema de impulso 2 para Launch attack (prototipo B)
  (Pawn|Components|CharacterMovement|SetMovementMode (Variables|Character|GetCharacterMovement) "MOVE_Falling" 0)
  (Character|LaunchCharacter (* (Transformation|GetActorForwardVector) (Utilities|Select :Index (Variables|Default|GetComboIndex) :Option%200 1e+03 :Option%201 9e+02)) true false))

(event Custom|Disable_Hitbox_R
  ;[0.02423 0 1] Hit_box (test)
  (Collision|SetCollisionEnabled (Variables|Default|GetHitbox_RightHand) "NoCollision")
  (Utilities|Array|Clear (Variables|Default|Getenemies_hit)))

(event Custom|Enable_Hitbox_R
  ;[0.02423 0 1] Hit_box (test)
  (Collision|SetCollisionEnabled (Variables|Default|GetHitbox_RightHand) "QueryOnly"))

(event Custom|Deal_Damage_To_Enemy
  (params (Enemy_Actor :type Actor%20Object%20Reference))
  ;[0.02423 0 1] Hit_box (test)
  (if (not (Utilities|Array|ContainsItem (Variables|Default|Getenemies_hit) 0))
    (Game|Damage|ApplyDamage Enemy_Actor (Variables|Default|GetCurrent_Attack_Damage) 0 self)
    (Utilities|Array|Add (Variables|Default|Getenemies_hit) 0)
    (if (>= (Variables|Default|GetCurrent_Attack_Damage) 6.0)
      (Game|Feedback|ClientStartCameraShake (Game|GetPlayerController 0) "/Game/Project_D/Blueprints/BP_HeavyHit_Shake.BP_HeavyHit_Shake_C" 1.0 "CameraLocal" "0, 0, 0"))))

(event Custom|Enable_Hitbox_L
  ;[0.02423 0 1] Hit_box (test)
  (Collision|SetCollisionEnabled (Variables|Default|GetHitbox_LeftHand) "QueryOnly"))

(event Custom|Disable_Hitbox_L
  ;[0.02423 0 1] Hit_box (test)
  (Collision|SetCollisionEnabled (Variables|Default|GetHitbox_LeftHand) "NoCollision")
  (Utilities|Array|Clear (Variables|Default|Getenemies_hit)))

(event Custom|AbrirCombo
  (bind _mesh (Variables|Character|GetMesh))
  (bind _mesh_2 (Variables|Character|GetMesh))
  ;[1 0.2732 0.6039] Quick_Attack
  (Utilities|FlowControl|Sequence
    (:then_0
      (Utilities|FlowControl|DoOnce false) ; enters at Reset
    )
    (:then_1
      ;[0 1 0.07624] Launch_Attack
      (Utilities|FlowControl|DoOnce false) ; enters at Reset
    )))

(event Input|EnhancedActionEvents|EnhancedInputActionIA_Move
  (params (ActionValue :type Vector%202D%20Structure) (ElapsedSeconds :type Float%20%28double-precision%29) (TriggeredSeconds :type Float%20%28double-precision%29) (InputAction :type Input%20Action%20Object%20Reference :default "/Game/Project_D/Inputs/IA_Move.IA_Move"))
  (bind _returnvalue (Transformation|GetActorLocation))
  (bind _returnvalue_2 (Math|Vector|MakeVector (.x ActionValue) (.y ActionValue) 0.0))
  (bind _targetcamera (Variables|Default|GetTargetCamera))
  (bind _returnvalue_3 (Actor|GetComponentbyClass _targetcamera "/Script/Engine.CameraComponent"))
  (bind _returnvalue_4 (Math|Vector|VectorLength _returnvalue_2))
  (bind _returnvalue_5 (Transformation|GetWorldLocation _returnvalue_3))
  (bind _returnvalue_6 (> _returnvalue_4 0.8))
  (bind _returnvalue_7 (Math|Float|SelectFloat 1.0 0.25 _returnvalue_6))
  (bind _returnvalue_8 (Math|Rotator|FindLookatRotation _returnvalue _returnvalue_5))
  (bind _returnvalue_9 (Math|Vector|GetRightVector _returnvalue_8))
  (bind (_x _y) (Math|Vector|BreakVector _returnvalue_9))
  ;[1 0.9958 0.5284] MK: Shaolin Monks–style movement system
  ;;[1 0.155 0.5825] Deshabilita el movimiento durante el combo
  (if (not (Variables|Default|GetIsComboActive?))
    (if (not (Variables|Default|GetIsHanging))
      (Pawn|Input|AddMovementInput (Math|Vector|Normalize (Math|Vector|GetForwardVector _returnvalue_8)) (* (* (.x ActionValue) _returnvalue_7) -1.0) false)
      (Pawn|Input|AddMovementInput (Math|Vector|Normalize (Math|Vector|MakeVector _x _y 0.0)) (* (* (.y ActionValue) _returnvalue_7) -1.0) false))))

(event Input|EnhancedActionEvents|EnhancedInputActionIA_Attack
  (params (ActionValue :type Boolean) (ElapsedSeconds :type Float%20%28double-precision%29) (TriggeredSeconds :type Float%20%28double-precision%29) (InputAction :type Input%20Action%20Object%20Reference :default "/Game/Project_D/Inputs/IA_Attack.IA_Attack"))
  (bind _mesh (Variables|Character|GetMesh))
  ;[1 0.2732 0.6039] Quick_Attack
  (:Started
    (Development|PrintString "QUICK ATTACK!" true true "(R=0.407240,G=0.111932,B=0.246201,A=1.000000)" 1.0)
    (Utilities|FlowControl|DoOnce false :!label _label
      (:Completed
        (Variables|Default|SetIsComboActive? true)
        (Variables|Default|SetCurrent_Attack_Damage (Utilities|Select :Index (Variables|Default|GetComboIndex) :Option%200 5.0 :Option%201 5.0 :Option%202 6.0))
        (Development|PrintString (Utilities|String|ToString(Float) (* (Variables|Default|GetCurrent_Attack_Damage) -1.0)) true true "(R=0.991102,G=0.000000,B=0.651406,A=1.000000)" 3.0)
        (if (== (Variables|Default|GetComboIndex) 0)
          (Animation|Montage|PlayMontage _mesh "/Game/Project_D/Characters/Leena/Animations/AM_Combat.AM_Combat" 1.0 0.0 (Utilities|Select :Index (Variables|Default|GetComboIndex) :Option%200 "Combo1" :Option%201 "Combo2" :Option%202 "Combo3") :!label _label_2
            (:then
              (CallFunction|QuickAttackImpulse)
              (Variables|Default|SetComboIndex (+ (Variables|Default|GetComboIndex) 1))
              (Pawn|Components|CharacterMovement|SetMovementMode (Variables|Character|GetCharacterMovement) "MOVE_Walking" 0 :!label _label_3))
            (:OnCompleted
              (Variables|Default|SetComboIndex 0 :!label _label_4)
              (Variables|Default|SetIsComboActive? false))
            (:OnBlendOut
              (goto _label Reset)))
          (else
            (bind _isbackwards_ (CallFunction|CheckAttackDirection))
            (if _isbackwards_
              (goto _label_2)
              (else
                (Animation|Montage|PlayMontage _mesh "/Game/Project_D/Characters/Leena/Animations/AM_Combat.AM_Combat" 1.0 0.0 (Utilities|Select :Index (Variables|Default|GetComboIndex) :Option%200 "Combo1" :Option%201 "Combo2" :Option%202 "Combo3")
                  (:then
                    (CallFunction|QuickAttackImpulse)
                    (Variables|Default|SetComboIndex (+ (Variables|Default|GetComboIndex) 1))
                    (if (>= (Variables|Default|GetComboIndex) 3)
                      (Variables|Default|SetComboIndex 0)
                      (goto _label_3)
                      (else
                        (goto _label_3))))
                  (:OnCompleted
                    (goto _label_4))
                  (:OnBlendOut
                    (goto _label Reset)))))))))))

(event Input|EnhancedActionEvents|EnhancedInputActionIA_Jump
  (params (ActionValue :type Boolean) (ElapsedSeconds :type Float%20%28double-precision%29) (TriggeredSeconds :type Float%20%28double-precision%29) (InputAction :type Input%20Action%20Object%20Reference :default "/Game/Project_D/Inputs/IA_Jump.IA_Jump"))
  (bind _returnvalue (Transformation|GetActorForwardVector))
  (bind _returnvalue_2 (Transformation|GetActorRotation))
  (bind _returnvalue_3 (Class|Pawn|GetLastMovementInputVector))
  (bind _mesh (Variables|Character|GetMesh))
  (bind _returnvalue_4 (Class|KismetAnimationLibrary|CalculateDirection _returnvalue_3 _returnvalue_2))
  ;[1 1 1] System Jump (Chupala pery)
  (:Started
    (if (Variables|Default|GetIsHanging)
      (Utilities|FlowControl|DoOnce false :!label _label
        (:Completed
          (Variables|Default|SetCanWallGrab? false)
          (Animation|PlayAnimMontage "/Game/Project_D/Characters/Leena/Animations/anim_ledge_climbFlip_Montage.anim_ledge_climbFlip_Montage" 1.0 "None")
          (Character|LaunchCharacter (+ _returnvalue "0.000000,0.000000,1500.000000") false false)
          (Utilities|FlowControl|Delay 0.25)
          (Character|LaunchCharacter (* _returnvalue 225.0) false false)
          (Variables|Default|SetIsHanging false)
          (Variables|Default|SetCanWallGrab? true)
          (goto _label Reset)))
      (else
        ;[0.08993 0.9203 1 0.466] Lock On System (apuntado prototype)
        (if (Variables|Default|GetIsLockedOn)
          (Development|PrintString "INTENTO DE DASH" true true "(R=0.040713,G=0.404800,B=0.619792,A=1.000000)")
          (if (> (Math|Vector|VectorLength _returnvalue_3) 0.1)
            (if (Math|Float|InRange(Float) _returnvalue_4 -45.0 45.0)
              ;[1 1 1] NORTE, SUR, ESTE Y OESTE (EVADE_DASH_SYSTEM)
              (Character|LaunchCharacter (* (Transformation|GetActorForwardVector) (Variables|Default|GetDash_Force)) true true)
              (Animation|Montage|PlayMontage _mesh "/Game/Project_D/Characters/Leena/Animations/Dash_Lock_On/AM_anim_dash2_north_Montage.AM_anim_dash2_north_Montage")
              (elif (Math|Float|InRange(Float) _returnvalue_4 45.0 135.0)
                (Character|LaunchCharacter (* (Transformation|GetActorRightVector) (Variables|Default|GetDash_Force)) true true)
                (Animation|Montage|PlayMontage _mesh "/Game/Project_D/Characters/Leena/Animations/Dash_Lock_On/am_anim_dash2_east_Montage.am_anim_dash2_east_Montage")
                (elif (Math|Float|InRange(Float) _returnvalue_4 -135.0 -45.0)
                  (Character|LaunchCharacter (* (Transformation|GetActorRightVector) (* (Variables|Default|GetDash_Force) -1.0)) true true)
                  (Animation|Montage|PlayMontage _mesh "/Game/Project_D/Characters/Leena/Animations/Dash_Lock_On/AM_anim_dash2_west_Montage.AM_anim_dash2_west_Montage")
                  (else
                    (Character|LaunchCharacter (* (Transformation|GetActorForwardVector) (* (Variables|Default|GetDash_Force) -1.0)) true true :!label _label_2)
                    (Animation|Montage|PlayMontage _mesh "/Game/Project_D/Characters/Leena/Animations/Dash_Lock_On/am_dash2_south_Montage.am_dash2_south_Montage")))))
            (else
              (goto _label_2)))
          (else
            (Character|Jump))))))
  (:Completed
    (Character|StopJumping)))

(event Input|EnhancedActionEvents|EnhancedInputActionIA_LockOn
  (params (ActionValue :type Boolean) (ElapsedSeconds :type Float%20%28double-precision%29) (TriggeredSeconds :type Float%20%28double-precision%29) (InputAction :type Input%20Action%20Object%20Reference :default "/Game/Project_D/Inputs/IA_LockOn.IA_LockOn"))
  ;[0.08993 0.9203 1 0.466] Lock On System (apuntado prototype)
  (:Triggered
    (Rendering|Debug|DrawDebugSphere (Transformation|GetActorLocation) 5e+02 12 "(R=0.000000,G=1.000000,B=0.074347,A=1.000000)" 2.0 2.0)
    (bind _outactors (Collision|SphereOverlapActors (Transformation|GetActorLocation) 5e+02 (Utilities|Array|MakeArray "ObjectTypeQuery3") "/Game/Project_D/Characters/Oni/Blueprints/BP_Oni.BP_Oni_C"))
    (Utilities|IsValid (Utilities|Array|Get(acopy) _outactors)
      (:Is%20Valid
        (Variables|Default|SetLockedTarget (Utilities|Array|Get(acopy) _outactors))
        (Variables|Default|SetIsLockedOn true)
        (Variables|/Script/Engine.CharacterMovementComponent|SetMaxWalkSpeed (Variables|Character|GetCharacterMovement) 2.5e+02)
        (Variables|Default|SetbUseControllerRotationYaw true))
      (:Is%20Not%20Valid
        (Development|PrintString "No enemys detected"))))
  (:Completed
    (Variables|Default|SetIsLockedOn false)
    (Variables|Default|SetbUseControllerRotationYaw false)
    (Variables|/Script/Engine.CharacterMovementComponent|SetMaxWalkSpeed (Variables|Character|GetCharacterMovement) 6e+02)
    (Variables|Default|SetLockedTarget 0)))

(event Input|EnhancedActionEvents|EnhancedInputActionIA_Attack_Power
  (params (ActionValue :type Boolean) (ElapsedSeconds :type Float%20%28double-precision%29) (TriggeredSeconds :type Float%20%28double-precision%29) (InputAction :type Input%20Action%20Object%20Reference :default "/Game/Project_D/Inputs/IA_Attack_Power.IA_Attack_Power"))
  ;[1 0 0] Power_attack
  (:Started
    ;;[0.2 0 0] ¡Running Power Attack!
    (if (> (Math|Vector|VectorLength (Variables|/Script/Engine.MovementComponent|GetVelocity (Variables|Character|GetCharacterMovement))) 5e+02)
      (Development|PrintString "RUNNING POWER ATTACK!" true true "(R=1.000000,G=0.000000,B=0.025346,A=1.000000)" 1.0)
      (Variables|Default|SetIsComboActive? true)
      (Variables|Default|SetCurrent_Attack_Damage 3e+01)
      (Animation|Montage|PlayMontage (Variables|Character|GetMesh) "/Game/Project_D/Characters/Leena/Animations/AM_ChoyLayFut_SprintKick_Montage.AM_ChoyLayFut_SprintKick_Montage"
        (:then
          (Character|LaunchCharacter (* (Transformation|GetActorForwardVector) 2.5e+03) true true))
        (:OnCompleted
          (Variables|Default|SetIsComboActive? false :!label _label)
          (Pawn|Components|CharacterMovement|SetMovementMode (Variables|Character|GetCharacterMovement) "MOVE_Walking" 0))
        (:OnInterrupted
          (goto _label)))
      (else
        (Development|PrintString "POWER ATTACK!" true true "(R=1.000000,G=0.000000,B=0.025346,A=1.000000)" 1.0)
        (Utilities|FlowControl|DoOnce false :!label _label_2
          (:Completed
            (Variables|Default|SetIsComboActive? true)
            (Variables|Default|SetCurrent_Attack_Damage 28.0)
            (Development|PrintString (Utilities|String|ToString(Float) (* (Variables|Default|GetCurrent_Attack_Damage) -1.0)) true true "(R=0.991102,G=0.000000,B=0.651406,A=1.000000)" 3.0)
            (Animation|Montage|PlayMontage (Variables|Character|GetMesh) "/Game/Project_D/Characters/Leena/Animations/AM_ChoyLayFut_PowerPunch_A_north.AM_ChoyLayFut_PowerPunch_A_north"
              (:then
                (Character|LaunchCharacter (* (Transformation|GetActorForwardVector) 2.5e+03) true true))
              (:OnCompleted
                (Variables|Default|SetIsComboActive? false :!label _label_3)
                (Pawn|Components|CharacterMovement|SetMovementMode (Variables|Character|GetCharacterMovement) "MOVE_Walking" 0))
              (:OnBlendOut
                (goto _label_2 Reset))
              (:OnInterrupted
                (goto _label_3)))))))))

(event Input|EnhancedActionEvents|EnhancedInputActionIA_Attack_Launch
  (params (ActionValue :type Boolean) (ElapsedSeconds :type Float%20%28double-precision%29) (TriggeredSeconds :type Float%20%28double-precision%29) (InputAction :type Input%20Action%20Object%20Reference :default "/Game/Project_D/Inputs/IA_Attack_Launch.IA_Attack_Launch"))
  (bind _mesh (Variables|Character|GetMesh))
  ;[0 1 0.07624] Launch_Attack
  (:Started
    (Development|PrintString "LAUNCH ATTACK!" true true "(R=0.000000,G=1.000000,B=0.036073,A=1.000000)" 1.0)
    (Utilities|FlowControl|DoOnce false :!label _label
      (:Completed
        (Variables|Default|SetIsComboActive? true)
        (Pawn|Components|CharacterMovement|SetMovementMode (Variables|Character|GetCharacterMovement) "MOVE_None" 0)
        (Variables|Default|SetCurrent_Attack_Damage (Utilities|Select :Index (Variables|Default|GetComboIndex) :Option%200 1e+01 :Option%201 12.0))
        (Development|PrintString (Utilities|String|ToString(Float) (* (Variables|Default|GetCurrent_Attack_Damage) -1.0)) true true "(R=0.000000,G=0.407240,B=0.030713,A=1.000000)" 3.0)
        (if (== (Variables|Default|GetComboIndex) 0)
          (Animation|Montage|PlayMontage _mesh "/Game/Project_D/Characters/Leena/Animations/Kempo/AM_Kempo_uppercuts.AM_Kempo_uppercuts" 1.0 0.0 (Utilities|Select :Index (Variables|Default|GetComboIndex) :Option%200 "Combo1" :Option%201 "Combo2") :!label _label_2
            (:then
              (CallFunction|LaunchAttackImpulse)
              (Variables|Default|SetComboIndex (+ (Variables|Default|GetComboIndex) 1))
              (Pawn|Components|CharacterMovement|SetMovementMode (Variables|Character|GetCharacterMovement) "MOVE_Walking" 0 :!label _label_3))
            (:OnCompleted
              (Variables|Default|SetComboIndex 0 :!label _label_4)
              (Variables|Default|SetIsComboActive? false))
            (:OnBlendOut
              (goto _label Reset)))
          (else
            (bind _isbackwards_ (CallFunction|CheckAttackDirection))
            (if _isbackwards_
              (goto _label_2)
              (else
                (Animation|Montage|PlayMontage _mesh "/Game/Project_D/Characters/Leena/Animations/Kempo/AM_Kempo_uppercuts.AM_Kempo_uppercuts" 1.0 0.0 (Utilities|Select :Index (Variables|Default|GetComboIndex) :Option%200 "Combo1" :Option%201 "Combo2")
                  (:then
                    (CallFunction|LaunchAttackImpulse)
                    (Variables|Default|SetComboIndex (+ (Variables|Default|GetComboIndex) 1))
                    (if (>= (Variables|Default|GetComboIndex) 2)
                      (Variables|Default|SetComboIndex 0)
                      (goto _label_3)
                      (else
                        (goto _label_3))))
                  (:OnCompleted
                    (goto _label_4))
                  (:OnBlendOut
                    (goto _label Reset)))))))))))

(event EventBeginPlay
  ;[0 0 0] ¿Camara system?
  (bind _returnvalue (Actor|GetActorOfClass "/Game/Project_D/Blueprints/BP_CineCamera_Manager.BP_CineCamera_Manager_C"))
  (Variables|Default|SetTargetCamera _returnvalue)
  (Input|AddMappingContext (PlayerController|LocalPlayerSubsystems|GetEnhancedInputLocalPlayerSubsystem (Game|GetPlayerController 0)) "/Game/Project_D/Inputs/IMC_Leena.IMC_Leena" 0 "(bIgnoreAllPressedKeysUntilRelease=True,bForceImmediately=False,bNotifyUserSettings=False)"))

(event EventTick
  (params (DeltaSeconds :type Float%20%28single-precision%29))
  (bind _returnvalue (Game|GetPlayerController 0))
  (Utilities|FlowControl|Sequence
    (:then_0
      (CallFunction|DetectLedge))
    (:then_1
      (if (Variables|Default|GetIsLockedOn)
        (Utilities|IsValid (Variables|Default|GetLockedTarget)
          (:Is%20Valid
            (if (> (Transformation|GetDistanceTo (Variables|Default|GetLockedTarget) self) 1.5e+03)
              (Variables|Default|SetIsLockedOn false)
              (Variables|/Script/Engine.CharacterMovementComponent|SetMaxWalkSpeed (Variables|Character|GetCharacterMovement) 6e+02)
              (Variables|Default|SetbUseControllerRotationYaw false)
              (else
                (Pawn|SetControlRotation _returnvalue (Math|Interpolation|RInterpTo (Pawn|GetControlRotation _returnvalue :!class /Script/Engine.Controller) (Math|Rotator|FindLookatRotation (Transformation|GetActorLocation) (Transformation|GetActorLocation (Variables|Default|GetLockedTarget))) (Utilities|Time|GetWorldDeltaSeconds) 5.0))))))))))

(event Input|KeyboardEvents|P
  (params (Key :type Key%20Structure :default "None"))
  ;[1 1 1] Debug Mode (Press "P" para ver lineas y esas cosas)
  (:Pressed
    (Utilities|FlowControl|FlipFlop
      (:A
        (Variables|Default|SetDebugMode true))
      (:B
        (Variables|Default|SetDebugMode false)))))

(fn ConstructionScript)

(fn DetectLedge
  (bind _returnvalue (Transformation|GetActorLocation))
  (bind _returnvalue_2 (+ _returnvalue "0.000000,0.000000,50.000000"))
  (if (not (Variables|Default|GetIsHanging))
    (bind (_outhit _returnvalue_3) (Collision|LineTraceByChannel _returnvalue_2 (+ _returnvalue_2 (* (Transformation|GetActorForwardVector) 1e+02)) "TraceTypeQuery1" false 0 (select (Variables|Default|GetDebugMode) "ForDuration" "None")))
    (if _returnvalue_3
      (if (Actor|ActorHasTag (.HitActor (Collision|BreakHitResult _outhit)) "Ledge")
        (Transformation|SetActorRotation (Math|Rotator|MakeRotator 0.0 0.0 (.yaw (Math|Rotator|MakeRotfromX (* (.ImpactNormal (Collision|BreakHitResult _outhit)) -1.0)))))
        (if true
          (bind (_outhit_2 _returnvalue_4) (Collision|LineTraceByChannel (+ (+ (.ImpactPoint (Collision|BreakHitResult _outhit)) (* (.ImpactNormal (Collision|BreakHitResult _outhit)) -3.0)) "0.000000,0.000000,60.000000") (- (+ (+ (.ImpactPoint (Collision|BreakHitResult _outhit)) (* (.ImpactNormal (Collision|BreakHitResult _outhit)) -3.0)) "0.000000,0.000000,60.000000") "0.000000,0.000000,100.000000") "TraceTypeQuery1" false 0 (select (Variables|Default|GetDebugMode) "ForDuration" "None") true "(R=0.049641,G=0.000000,B=1.000000,A=1.000000)"))
          (if _returnvalue_4
            (if (Actor|ActorHasTag (.HitActor (Collision|BreakHitResult _outhit_2)) "Ledge")
              (bind _output_get (Variables|Default|SetTargetGripLocation (.ImpactPoint (Collision|BreakHitResult _outhit_2))))
              (Rendering|Debug|DrawDebugSphere _output_get 0.0 12 "(R=1.000000,G=0.000000,B=0.850150,A=1.000000)" 0.1)
              (Pawn|Components|CharacterMovement|SetMovementMode (Variables|Character|GetCharacterMovement) "MOVE_Flying" 0)
              (Components|Movement|StopMovementImmediately (Variables|Character|GetCharacterMovement))
              (Variables|Default|SetIsHanging true)
              (Transformation|SetActorLocation (- (+ (.ImpactPoint (Collision|BreakHitResult _outhit_2)) (* (.ImpactNormal (Collision|BreakHitResult _outhit)) 55.0)) "0.000000,0.000000,61.000000") false true))))))))

(fn CheckAttackDirection)

(fn ForceResetHitboxes
  (Utilities|FlowControl|Sequence
    (:then_0
      (Collision|SetCollisionEnabled (Variables|Default|GetHitbox_RightHand) "NoCollision"))
    (:then_1
      (Collision|SetCollisionEnabled (Variables|Default|GetHitbox_LeftHand) "NoCollision")))
  (Utilities|Array|Clear (Variables|Default|Getenemies_hit)))