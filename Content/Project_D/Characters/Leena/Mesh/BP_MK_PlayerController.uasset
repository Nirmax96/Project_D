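; Player controller for Leena that adds an Enhanced Input mapping context on BeginPlay and handles level and character reset inputs.
; The level reset reopens the current level by name.
; The character reset destroys the controlled pawn, then spawns and possesses a new BP_Leena at the first actor tagged RespawnLeena.
; It does nothing if no tagged actor or valid pawn exists.
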(event Input|EnhancedActionEvents|EnhancedInputActionIA_ResetLevel
  (params (ActionValue :type Boolean) (ElapsedSeconds :type Float%20%28double-precision%29) (TriggeredSeconds :type Float%20%28double-precision%29) (InputAction :type Input%20Action%20Object%20Reference :default "/Game/Project_D/Inputs/DebugInputs/IA_ResetLevel.IA_ResetLevel"))
  (:Started
    (bind _returnvalue (Game|GetCurrentLevelName true))
    (Game|OpenLevel(byName) (Utilities|String|StringToName _returnvalue))))

(event Input|EnhancedActionEvents|EnhancedInputActionIA_ResetCharacter
  (params (ActionValue :type Boolean) (ElapsedSeconds :type Float%20%28double-precision%29) (TriggeredSeconds :type Float%20%28double-precision%29) (InputAction :type Input%20Action%20Object%20Reference :default "/Game/Project_D/Inputs/DebugInputs/IA_ResetCharacter.IA_ResetCharacter"))
  (:Started
    (Variables|Default|SetOldPawn (Pawn|GetControlledPawn))
    (bind _outactors (Actor|GetAllActorswithTag "RespawnLeena"))
    (if (> (Utilities|Array|Length _outactors) 0)
      (Utilities|IsValid (Variables|Default|GetOldPawn)
        (:Is%20Valid
          (Pawn|UnPossess)
          (Actor|DestroyActor (Variables|Default|GetOldPawn))
          (bind _returnvalue (Game|SpawnActorfromClass "/Game/Project_D/Characters/Leena/Blueprints/BP_Leena.BP_Leena_C" (Transformation|GetActorTransform (Utilities|Array|Get(acopy) _outactors)) "Undefined" "MultiplyWithRoot" 0 0))
          (Pawn|Possess _returnvalue))))))

(event EventBeginPlay
  (Input|AddMappingContext (PlayerController|LocalPlayerSubsystems|GetEnhancedInputLocalPlayerSubsystem self) 0 0 "(bIgnoreAllPressedKeysUntilRelease=True,bForceImmediately=False,bNotifyUserSettings=False)"))

(fn ConstructionScript)