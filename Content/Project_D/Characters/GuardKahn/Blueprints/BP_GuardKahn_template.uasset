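; GuardKahn template Blueprint for a modular guard character with toggleable equipment: lance, claws, helmet, shoulder pads, belts and other armor pieces.
; The construction script makes each equipment skeletal mesh follow the main Mesh through a leader pose component, so all pieces share its animation.
; A boolean per piece then sets that piece's visibility, allowing different loadouts to be configured per instance or variant.
; The event graph holds no active logic.
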(event EventBeginPlay)

(event Collision|EventActorBeginOverlap
  (params (OtherActor :type Actor%20Object%20Reference)))

(event EventTick
  (params (DeltaSeconds :type Float%20%28single-precision%29)))

(fn ConstructionScript
  (Components|SkinnedMesh|SetLeaderPoseComponent (Variables|Default|GetSK_lance) (Variables|Character|GetMesh) false false)
  (Rendering|SetVisibility (Variables|Default|GetSK_Helmet) (Variables|E_Head|GetHelmet) false)
  (Rendering|SetVisibility (Variables|Default|GetSK_lance) (Variables|WEAPONS|GetLance) false)
  (Rendering|SetVisibility (Variables|Default|GetSK_garra_L) (Variables|B_Arm_L|GetGarra_L) false)
  (Rendering|SetVisibility (Variables|Default|GetSK_garra_R) (Variables|A_Arm_R|GetGarra_R) false)
  (Rendering|SetVisibility (Variables|Default|GetSK_hombreras_L) (Variables|B_Arm_L|GetHombreras_L) false)
  (Rendering|SetVisibility (Variables|Default|GetSK_hombreras_R) (Variables|A_Arm_R|GetHombreras_R) false)
  (Rendering|SetVisibility (Variables|Default|GetSK_protect_front) (Variables|C_Legs|GetProtect_Front) false)
  (Rendering|SetVisibility (Variables|Default|GetSK_protect_laterals) (Variables|C_Legs|GetProtect_Laterals) false)
  (Rendering|SetVisibility (Variables|Default|GetSK_rodilleras) (Variables|C_Legs|GetRodilleras) false)
  (Rendering|SetVisibility (Variables|Default|GetSK_canilleras) (Variables|C_Legs|GetCanilleras) false)
  (Rendering|SetVisibility (Variables|Default|GetSK_codera_L) (Variables|B_Arm_L|GetCodera_L) false)
  (Rendering|SetVisibility (Variables|Default|GetSK_codera_R) (Variables|A_Arm_R|GetCodera_R) false)
  (Rendering|SetVisibility (Variables|Default|GetSK_cinto) (Variables|C_Legs|GetCinto) false)
  (Rendering|SetVisibility (Variables|Default|GetSK_cinturones) (Variables|D_Torso|GetCinturones) false)
  (Rendering|SetVisibility (Variables|Default|GetSK_antebrazo_R) (Variables|A_Arm_R|Getantebrazo_R) false)
  (Rendering|SetVisibility (Variables|Default|GetSK_antebrazo_L) (Variables|B_Arm_L|Getantebrazo_L) false))