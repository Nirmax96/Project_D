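; BP_DragonKoin is a coin pickup that spawns a BP_Oni enemy when Leena overlaps its trigger zone.
; The Oni spawns at the TargetSpawnPoint's transform with Leena as owner, and a pickup sound plays.
; The coin then hides and disables its trigger, a step marked as testing-only, and reappears through ResetKoin when that Oni's died event fires.
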(event OnComponentBeginOverlap(TriggerZone)
  (params (OverlappedComponent :type Primitive%20Component%20Object%20Reference) (OtherActor :type Actor%20Object%20Reference) (OtherComp :type Primitive%20Component%20Object%20Reference) (OtherBodyIndex :type Integer) (bFromSweep :type Boolean) (SweepResult :type Hit%20Result%20Structure%20%28by%20ref%29))
  (bind _asbp_leena (Utilities|Casting|CastToBP_Leena OtherActor))
  (bind _returnvalue (Game|SpawnActorfromClass "/Game/Project_D/Characters/Oni/Blueprints/BP_Oni.BP_Oni_C" (Transformation|GetActorTransform (Variables|Default|GetTargetSpawnPoint)) "Undefined" "MultiplyWithRoot" _asbp_leena 0))
  (Audio|PlaySoundatLocation "/Game/Project_D/Sounds/Coin_Sounds/SFX_KoinPickup.SFX_KoinPickup" (Transformation|GetActorLocation) "0, 0, 0" 1.0 1.0 0.0 0 0 0 0)
  ;[1 1 1] SOLO PARA TESTING
  (Rendering|SetActorHiddenInGame self true)
  (Collision|SetCollisionEnabled (Variables|Default|GetTriggerZone) "NoCollision")
  (EventDispatchers|BindEventtoOniDied _returnvalue (delegate Custom|ResetKoin)))

(event Custom|ResetKoin
  ;[1 1 1] SOLO PARA TESTING
  (Rendering|SetActorHiddenInGame self false)
  (Collision|SetCollisionEnabled (Variables|Default|GetTriggerZone) "QueryAndPhysics"))

(fn ConstructionScript)