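; Blueprint controller that plays a Level Sequence cutscene while suspending the player's move and look input.
; CutscenePlayer ignores repeat calls during playback, creates a sequence player, switches the view to the cutscene camera and binds an event to the sequence's finish.
; AfterPlay blends the view to a return camera, restores input, clears the playing flag and prints a debug message.
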(event Custom|AfterPlay
  (bind _returnvalue (Game|GetPlayerController 0))
  (Game|Player|SetViewTargetwithBlend (Game|GetPlayerController 0) (Variables|Default|GetReturnCamera) (Variables|Default|GetBlendTime) "VTBlend_Linear" 0.0 false)
  (Input|SetIgnoreMoveInput _returnvalue false)
  (Input|SetIgnoreLookInput _returnvalue false)
  (Variables|Default|SetIsPlaying false)
  (Development|PrintString "Finished  Playing"))

(event Custom|CutscenePlayer
  (bind _returnvalue (Game|GetPlayerController 0))
  (if (not (Variables|Default|GetIsPlaying))
    (Variables|Default|SetIsPlaying true)
    (bind _returnvalue_2 (Sequencer|Player|CreateLevelSequencePlayer (Variables|Default|GetLevel%20Sequence)))
    (EventDispatchers|BindEventtoOnFinished _returnvalue_2 (EventDispatchers|CreateEvent :!event Custom|AfterPlay))
    (Input|SetIgnoreMoveInput _returnvalue true)
    (Input|SetIgnoreLookInput _returnvalue true)
    (Game|Player|SetViewTargetwithBlend _returnvalue (Variables|Default|GetCutsceneCamera) 0.0 "VTBlend_Linear" 0.0 false)
    (Sequencer|Player|Play _returnvalue_2 :!class /Script/MovieScene.MovieSceneSequencePlayer)))

(fn ConstructionScript)