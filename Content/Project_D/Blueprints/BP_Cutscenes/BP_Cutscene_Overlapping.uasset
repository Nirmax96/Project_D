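; BP_Cutscene_Overlapping is a trigger that starts a cutscene when BP_Leena overlaps its Box component.
; It finds the level's BP_CutsceneController, passes it the level sequence, blend time and gameplay and cutscene cameras, then calls CutscenePlayer.
; IsReplayable allows repeat triggers; otherwise IsPlayed limits it to a single play.
; A missing controller only prints a message.
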(event OnComponentBeginOverlap(Box)
  (params (OverlappedComponent :type Primitive%20Component%20Object%20Reference) (OtherActor :type Actor%20Object%20Reference) (OtherComp :type Primitive%20Component%20Object%20Reference) (OtherBodyIndex :type Integer) (bFromSweep :type Boolean) (SweepResult :type Hit%20Result%20Structure%20%28by%20ref%29))
  (Utilities|Casting|CastToBP_Leena OtherActor)
  (if (Variables|Default|GetIsReplayable)
    (bind _returnvalue (Actor|GetActorOfClass "/Game/Project_D/Blueprints/BP_Cutscenes/BP_CutsceneController.BP_CutsceneController_C" :!label _label))
    (Utilities|IsValid _returnvalue
      (:Is%20Valid
        (Variables|/Game/Project_D/Blueprints/BP_Cutscenes/BP_CutsceneController.BP_CutsceneController_C|SetLevel%20Sequence _returnvalue (Variables|Default|GetCinematicSequence))
        (Variables|/Game/Project_D/Blueprints/BP_Cutscenes/BP_CutsceneController.BP_CutsceneController_C|SetBlendTime _returnvalue (Variables|Default|GetBlendTime))
        (Variables|/Game/Project_D/Blueprints/BP_Cutscenes/BP_CutsceneController.BP_CutsceneController_C|SetReturnCamera _returnvalue (Variables|Default|GetGameplayCamera))
        (Variables|/Game/Project_D/Blueprints/BP_Cutscenes/BP_CutsceneController.BP_CutsceneController_C|SetCutsceneCamera _returnvalue (Variables|Default|GetCameraCutscene))
        (Default|CutscenePlayer _returnvalue)
        (if (not (Variables|Default|GetIsReplayable))
          (Variables|Default|SetIsPlayed true)))
      (:Is%20Not%20Valid
        (Development|PrintString "No BP_CutsceneController Found" true true "(R=1.000000,G=0.000000,B=0.099285,A=1.000000)")))
    (elif (not (Variables|Default|GetIsPlayed))
      (goto _label))))

(event EventBeginPlay)

(fn ConstructionScript)