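; Combo component that counts hits, records the last enemy struck and drives the combo counter UI.
; Each registered hit increments the count, restarts a timeout timer and updates the UI from the second hit onward.
; Every tenth hit shows a milestone word from a clamped array lookup, while timeout resets count, target and UI.
; Pause and resume events let external callers freeze the timer, intended for launched, airborne enemies.
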(event Custom|StartComboTimer
  (Utilities|Time|ClearandInvalidateTimerbyHandle (Variables|Default|GetComboTimerHandle))
  (Utilities|Time|SetTimerbyEvent (delegate Custom|Event_TimeOut) 3.5))

(event Custom|Event_TimeOut
  (CallFunction|ResetCombo))

(event Custom|PauseComboTimer
  (Utilities|Time|PauseTimerbyHandle (Variables|Default|GetComboTimerHandle)))

(event Custom|ResumeComboTimer
  (Utilities|Time|UnpauseTimerbyHandle (Variables|Default|GetComboTimerHandle)))

(event Custom|RegisterHIT
  (params (HitEnemy :type Actor%20Object%20Reference))
  (bind _ui_reference (Variables|Default|GetUI_Reference))
  (CallFunction|AddComboHit HitEnemy)
  (CallFunction|StartComboTimer)
  (bind (_showmessage_ _messagetext) (CallFunction|CheckComboMilestone))
  (if (>= (Variables|Default|GetCurrentCombo) 2) ; Este branch evita que aparesca el "1"\ncomo primer golpe... \nse supone que el combo aparece apartir del 2
    (Widget|SetVisibility _ui_reference "Visible")
    (Default|UpdateText _ui_reference (Variables|Default|GetCurrentCombo) _messagetext _showmessage_)))

(fn AddComboHit
  (params (HitEnemy :type Actor%20Object%20Reference))
  (Variables|Default|SetCurrentTarget HitEnemy) ; Determina el enemigo al cual se le está atacando
  (Math|Integer|IncrementInt (Variables|Default|GetCurrentCombo)
    (:%20%20
      (if (>= (Variables|Default|GetCurrentCombo) 2) ; el golpe se suma y el "1" queda ignorado gracias a ese Branch.
        _))))

(fn CheckComboMilestone
  (if (== (Math|Integer|%(Integer) (Variables|Default|GetCurrentCombo) 10) 0)
    (return true (Utilities|Array|Get(acopy) (Variables|Default|GetComboWords) (Math|Integer|Clamp(Integer) (/ (Variables|Default|GetCurrentCombo) 10) 1 18)))
    (else
      (return false ""))))

(fn ResetCombo
  (Variables|Default|SetCurrentCombo 0)
  (Variables|Default|SetCurrentTarget 0)
  (Default|HideCombo (Variables|Default|GetUI_Reference)))