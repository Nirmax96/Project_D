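; Base player character Blueprint that handles analog, camera-relative locomotion through Enhanced Input.
; While CurrentState is Idle, IA_Move sets walk speed from a curve of stick magnitude and adds normalized movement input along the camera's right and forward vectors.
; It also interpolates player 0's control rotation from the actor's facing toward the input direction.
; A HasMoveInput flag tracks active input and clears when the action completes.
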(event EventBeginPlay)

(event Collision|EventActorBeginOverlap
  (params (OtherActor :type Actor%20Object%20Reference)))

(event EventTick
  (params (DeltaSeconds :type Float%20%28single-precision%29)))

(event Input|EnhancedActionEvents|EnhancedInputActionIA_Move
  (params (ActionValue :type Vector%202D%20Structure) (ElapsedSeconds :type Float%20%28double-precision%29) (TriggeredSeconds :type Float%20%28double-precision%29) (InputAction :type Input%20Action%20Object%20Reference :default "/Game/Project_D/Inputs/IA_Move.IA_Move"))
  (bind _returnvalue (Game|GetPlayerCameraManager 0))
  (bind _returnvalue_2 (Camera|GetCameraRotation _returnvalue))
  (bind (_roll _pitch _yaw) (Math|Rotator|BreakRotator _returnvalue_2))
  (bind _returnvalue_3 (Math|Vector|GetRightVector (Math|Rotator|MakeRotator _roll 0.0 _yaw)))
  (bind _returnvalue_4 (Math|Vector|GetForwardVector (Math|Rotator|MakeRotator 0.0 0.0 _yaw)))
  ;[0.2886 1 0.236] SISTEMA DE LOCOMOCIÓN: Lectura Analógica (Joystick/Teclado)
  (:Triggered
    (Variables|Input|SetAction%20Value%20X (.x ActionValue))
    (Variables|Input|SetAction%20Value%20Y (.y ActionValue))
    (if (CallFunction|CanMove)
      (Variables|Input|SetHas%20Move%20Input true)
      (Variables|/Script/Engine.CharacterMovementComponent|SetMaxWalkSpeed (Variables|Character|GetCharacterMovement) (Math|Curves|GetFloatValue (Variables|Default|GetSpeed_Curve) (Math|Vector2D|Vector2DLength (Math|Vector2D|MakeVector2D (Variables|Input|GetAction%20Value%20X) (Variables|Input|GetAction%20Value%20Y)))))
      ;;[0.9473 0.1045 0] APLICACIÓN DE FUERZA FÍSICA A LAS PIERNAS
      (Pawn|Input|AddMovementInput _returnvalue_3 (.x (Math|Vector2D|Normalize2D (Math|Vector2D|MakeVector2D (Variables|Input|GetAction%20Value%20X) (Variables|Input|GetAction%20Value%20Y)))) false) ; "Motor Lateral: Empuja al personaje hacia los costados \nde la cámara, usando la fuerza del eje X del joystick (Strafe)."
      (Pawn|Input|AddMovementInput _returnvalue_4 (.y (Math|Vector2D|Normalize2D (Math|Vector2D|MakeVector2D (Variables|Input|GetAction%20Value%20X) (Variables|Input|GetAction%20Value%20Y)))) false) ; "Motor Frontal: Empuja al personaje hacia donde \nmira la cámara, usando la fuerza del eje Y del joystick."
      (Pawn|SetControlRotation (Game|GetPlayerController 0) (Math|Interpolation|RInterpTo (Transformation|GetActorRotation) (Math|Rotator|MakeRotfromX (+ (* _returnvalue_3 (Variables|Input|GetAction%20Value%20X)) (* _returnvalue_4 (Variables|Input|GetAction%20Value%20Y)))) (Utilities|Time|GetWorldDeltaSeconds) 5.0))))
  (:Completed
    (Variables|Input|SetHas%20Move%20Input false)))

(fn ConstructionScript)

(fn CanMove
  (return (== (Variables|StateMachine|GetCurrentState) 0)) ; ¿El estado es Idle? Sí. Entonces te devuelvo un TRUE: podés moverte").
)