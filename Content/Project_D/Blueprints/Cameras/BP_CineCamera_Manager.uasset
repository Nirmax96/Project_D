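; Cine camera manager actor that moves its camera along a spline to follow the player character.
; Each tick it eases the camera toward the spline point nearest the player plus a smoothed offset, then snaps rotation to face the player.
; The offset tracks the player's X and Y deviation from the spline, with Y damped and constant biases, and no height component.
; The view-target switch to this actor is unconnected and never runs.
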(event EventTick
  (params (DeltaSeconds :type Float%20%28single-precision%29))
  (bind _returnvalue (Game|GetPlayerCharacter 0))
  (bind _camera (Variables|Default|GetCamera))
  (bind _spline (Variables|Default|GetSpline))
  (bind _returnvalue_2 (Transformation|GetWorldLocation _camera))
  (bind _returnvalue_3 (Transformation|GetActorLocation _returnvalue))
  (bind _returnvalue_4 (Spline|FindLocationClosesttoWorldLocation _spline _returnvalue_3 "World"))
  (bind _returnvalue_5 (- _returnvalue_3 _returnvalue_4))
  (bind (_x _y) (Math|Vector|BreakVector _returnvalue_5))
  (Transformation|SetWorldLocation _camera (Math|Interpolation|VInterpTo _returnvalue_2 (+ _returnvalue_4 (Variables|Default|GetCurrentOffset)) (Utilities|Time|GetWorldDeltaSeconds) 0.95) false false)
  (Transformation|SetWorldRotation _camera (Math|Rotator|FindLookatRotation _returnvalue_2 _returnvalue_3) false false)
  (Variables|Default|SetCurrentOffset (Math|Interpolation|VInterpTo (Variables|Default|GetCurrentOffset) (Math|Vector|MakeVector (- (* _x 1.0) 4e+02) (- (* _y 0.5) 5e+01) 0.0) (Utilities|Time|GetWorldDeltaSeconds) 2.0)))

(event EventBeginPlay)

(fn ConstructionScript)