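; Camera switch trigger that blends the player's view between a green-side and red-side camera as they cross a division line.
; While the player overlaps the box, a looping timer runs, checking their side via a dot product, with a threshold against flicker.
; A side change updates BP_CameraManager and snaps tracking cameras to the character.
; An unset camera falls back to the third-person character view, resetting control rotation.
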(event OnComponentBeginOverlap(Box)
  (params (OverlappedComponent :type Primitive%20Component%20Object%20Reference) (OtherActor :type Actor%20Object%20Reference) (OtherComp :type Primitive%20Component%20Object%20Reference) (OtherBodyIndex :type Integer) (bFromSweep :type Boolean) (SweepResult :type Hit%20Result%20Structure%20%28by%20ref%29))
  (if (== OtherActor (Game|GetPlayerCharacter 0))
    (if (Utilities|Time|IsValidTimerHandle (Variables|Default|GetTimerHandle))
      (Utilities|Time|UnpauseTimerbyHandle (Variables|Default|GetTimerHandle))
      (else
        (bind _returnvalue (Utilities|Time|SetTimerbyEvent (EventDispatchers|CreateEvent :!event Custom|TriggerCameraSwitch) 0.1 true))
        (Variables|Default|SetTimerHandle _returnvalue)))))

(event OnComponentEndOverlap(Box)
  (params (OverlappedComponent :type Primitive%20Component%20Object%20Reference) (OtherActor :type Actor%20Object%20Reference) (OtherComp :type Primitive%20Component%20Object%20Reference) (OtherBodyIndex :type Integer))
  (if (== OtherActor (Game|GetPlayerCharacter 0))
    (if (Utilities|Time|IsValidTimerHandle (Variables|Default|GetTimerHandle))
      (Utilities|Time|PauseTimerbyHandle (Variables|Default|GetTimerHandle)))))

(event Custom|TriggerCameraSwitch
  (bind _returnvalue (Game|GetPlayerCharacter 0))
  (bind _thirdpersonreference (Variables|References|GetThirdPersonReference))
  (bind _redsidecamera (Variables|RedSide|GetRedSideCamera))
  (bind _divisionline (Variables|Default|GetDivisionLine))
  (bind _greensidecamera (Variables|GreenSide|GetGreenSideCamera))
  (bind _returnvalue_2 (Transformation|GetActorLocation _returnvalue))
  (bind _returnvalue_3 (Transformation|GetWorldLocation _divisionline))
  (bind _returnvalue_4 (Math|Vector|GetForwardVector _divisionline))
  (bind _returnvalue_5 (- _returnvalue_2 _returnvalue_3))
  (bind _returnvalue_6 (Math|Vector|Normalize _returnvalue_5))
  (bind _returnvalue_7 (Math|Vector|DotProduct _returnvalue_6 _returnvalue_4))
  (bind _returnvalue_8 (Math|Float|Sign(Float) _returnvalue_7))
  (bind _returnvalue_9 (<= _returnvalue_8 0.0))
  (if (and (!= _returnvalue_8 (Variables|Default|GetPrevious%20side)) (> (Math|Float|Absolute(Float) _returnvalue_7) (Variables|Default|GetThreshold)))
    (Variables|Default|SetPrevious%20side _returnvalue_8)
    (Development|PrintString (Utilities|String|SelectString "green" "red" _returnvalue_9))
    (if _returnvalue_9
      (Utilities|IsValid _greensidecamera
        (:Is%20Valid
          (Game|Player|SetViewTargetwithBlend (Game|GetPlayerController 0) _greensidecamera (Variables|GreenSide|GetGreenBlendTime) "VTBlend_Linear" 0.0 false)
          (Default|SetActiveCamera (Variables|References|GetCameraManagerRefference) _greensidecamera)
          (if (Variables|/Game/Project_D/Blueprints/Cameras/BP_CameraBase.BP_CameraBase_C|GetIsTrackingCamera _greensidecamera)
            (Default|SnaptoCharacterView _greensidecamera)))
        (:Is%20Not%20Valid
          (Game|Player|SetViewTargetwithBlend (Game|GetPlayerController 0) _thirdpersonreference (Math|Float|SelectFloat (Variables|GreenSide|GetGreenBlendTime) (Variables|RedSide|GetRedBlendTime) _returnvalue_9) "VTBlend_Linear" 0.0 false :!label _label)
          (Default|SetActiveCamera (Variables|References|GetCameraManagerRefference) _thirdpersonreference)
          (Pawn|SetControlRotation (Game|GetPlayerController 0) (Transformation|GetActorRotation (Game|GetPlayerCharacter 0)))))
      (else
        (Utilities|IsValid _redsidecamera
          (:Is%20Valid
            (Game|Player|SetViewTargetwithBlend (Game|GetPlayerController 0) _redsidecamera (Variables|RedSide|GetRedBlendTime) "VTBlend_Linear" 0.0 false)
            (Default|SetActiveCamera (Variables|References|GetCameraManagerRefference) _redsidecamera)
            (if (Variables|/Game/Project_D/Blueprints/Cameras/BP_CameraBase.BP_CameraBase_C|GetIsTrackingCamera _redsidecamera)
              (Default|SnaptoCharacterView _redsidecamera)))
          (:Is%20Not%20Valid
            (goto _label)))))))

(event EventBeginPlay
  (Utilities|FlowControl|Sequence
    (:then_0
      (bind _asbp_leena (Utilities|Casting|CastToBP_Leena (Game|GetPlayerCharacter 0)))
      (Variables|References|SetThirdPersonReference _asbp_leena))
    (:then_1
      (bind _returnvalue (Actor|GetActorOfClass "/Game/Project_D/Blueprints/Cameras/BP_CameraManager.BP_CameraManager_C"))
      (Utilities|IsValid _returnvalue
        (:Is%20Valid
          (Variables|References|SetCameraManagerRefference _returnvalue))
        (:Is%20Not%20Valid
          (Development|PrintString "NoCameraManagerFound" true true "(R=1.000000,G=0.000000,B=0.060686,A=1.000000)"))))))

(event Collision|EventActorBeginOverlap
  (params (OtherActor :type Actor%20Object%20Reference)))

(event EventTick
  (params (DeltaSeconds :type Float%20%28single-precision%29)))

(fn ConstructionScript)