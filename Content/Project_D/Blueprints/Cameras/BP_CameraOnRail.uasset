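; Rail camera actor that follows the player character along a spline, with optional camera tracking.
; Each Tick finds the player's closest spline point, updates a speed-based rail distance using follow and look-ahead offsets, and interpolates Root there.
; RootPivot eases locally in XY toward the player by any excess beyond StartChasingDistance, ignoring Z.
; It prints the player's rail distance every frame and calls TrackingCamera when IsTrackingCamera is set.
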(event EventBeginPlay
  (|CallParentFunction) ; This node is disabled and will not be called.\nDrag off pins to build functionality.
)

(event Collision|EventActorBeginOverlap
  (params (OtherActor :type Actor%20Object%20Reference)))

(event EventTick
  (params (DeltaSeconds :type Float%20%28single-precision%29))
  (bind _returnvalue (Game|GetPlayerCharacter 0))
  (bind _rail (Variables|Default|GetRail))
  (bind _followoffset (Variables|Default|GetFollowOffset))
  (bind _rail_2 (Variables|Default|GetRail))
  (bind _followspeed (Variables|Default|GetFollowSpeed))
  (bind _delta_seconds (Variables|Default|GetDelta%20Seconds))
  (bind _rail_3 (Variables|Default|GetRail))
  (bind _returnvalue_2 (Spline|GetSplineLength _rail_3))
  (bind _returnvalue_3 (Spline|GetSplineLength _rail_2))
  (bind _returnvalue_4 (Transformation|GetActorLocation _returnvalue))
  (bind _returnvalue_5 (* _followspeed _delta_seconds))
  (bind _returnvalue_6 (Class|SplineComponent|FindInputKeyClosesttoWorldLocation _rail _returnvalue_4))
  (bind _returnvalue_7 (Class|SplineComponent|GetDistanceAlongSplineatSplineInputKey _rail _returnvalue_6))
  (bind _returnvalue_8 (+ _returnvalue_7 _followoffset))
  (bind _returnvalue_9 (Math|Float|Clamp(Float) _returnvalue_8 0.0 _returnvalue_2))
  (|CallParentFunction DeltaSeconds)
  ;[0.9563 1 0.3152] Obtiene el punto mas cercano del spline(riel) con el personaje
  (Variables|Default|SetClosestPointToPlayer (Class|SplineComponent|GetLocationatSplineInputKey (Variables|Default|GetRail) _returnvalue_6 "World"))
  (Variables|Default|SetCurrentDistance (Math|Float|Clamp(Float) (Math|Float|SelectFloat _returnvalue_9 (+ (* (Math|Float|Sign(Float) (- _returnvalue_9 (Variables|Default|GetCurrentDistance))) _returnvalue_5) (Variables|Default|GetCurrentDistance)) (<= (Math|Float|Absolute(Float) (- _returnvalue_9 (Variables|Default|GetCurrentDistance))) _returnvalue_5)) 0.0 _returnvalue_3))
  ;[0.4325 1 0.4263] Obtiene la distancia del personaje hasta el punto mas cercano al spline(riel)
  (Variables|Default|SetDistanceFromRail (Math|Vector|VectorLength (- (Transformation|GetActorLocation (Game|GetPlayerCharacter 0)) (Variables|Default|GetClosestPointToPlayer))))
  (Transformation|SetWorldLocation (Variables|Default|GetRoot) (Math|Interpolation|VInterpTo (Transformation|GetWorldLocation (Variables|Default|GetRoot)) (Spline|GetLocationatDistanceAlongSpline (Variables|Default|GetRail) (Math|Float|Clamp(Float) (+ (Variables|Default|GetCurrentDistance) (Variables|Default|GetLookAhead)) 0.0 _returnvalue_3) "World") (Variables|Default|GetDelta%20Seconds) (Variables|Default|GetInterp%20Speed)) false false)
  (Development|PrintString (Utilities|String|ToString(Float) (Variables|Default|GetDistanceFromRail)))
  (Transformation|SetRelativeLocation (Variables|Default|GetRoot_Pivot) (Math|Interpolation|VInterpTo (Variables|/Script/Engine.SceneComponent|GetRelativeLocation (Variables|Default|GetRoot_Pivot)) (select (and (> (- (Variables|Default|GetDistanceFromRail) (Variables|Default|GetStartChasingDistance)) 0.0) (> (Variables|Default|GetDistanceFromRail) 0.001)) (Math|Vector|MakeVector (.X (Math|Vector|BreakVector (Math|Transform|InverseTransformDirection (Transformation|GetWorldTransform (Variables|Default|GetRoot)) (* (- (Variables|Default|GetDistanceFromRail) (Variables|Default|GetStartChasingDistance)) (Math|Vector|Normalize (- (Transformation|GetActorLocation (Game|GetPlayerCharacter 0)) (Variables|Default|GetClosestPointToPlayer)) 0.01))))) (.Y (Math|Vector|BreakVector (Math|Transform|InverseTransformDirection (Transformation|GetWorldTransform (Variables|Default|GetRoot)) (* (- (Variables|Default|GetDistanceFromRail) (Variables|Default|GetStartChasingDistance)) (Math|Vector|Normalize (- (Transformation|GetActorLocation (Game|GetPlayerCharacter 0)) (Variables|Default|GetClosestPointToPlayer)) 0.01))))) 0.0) "0, 0, 0") (Variables|Default|GetDelta%20Seconds) (Variables|Default|GetInterp%20Speed)) false false)
  (if (Variables|Default|GetIsTrackingCamera)
    (CallFunction|TrackingCamera)))

(fn ConstructionScript
  (|CallParentFunction))