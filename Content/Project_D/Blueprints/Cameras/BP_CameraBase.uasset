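; Base camera actor that can act as a level's starting view and face the player character.
; On BeginPlay it finds BP_CameraManager and, if flagged as start camera, takes the view target, registers as active and optionally snaps its root toward the character.
; Tick disables the camera component's tick while another camera is active.
; An interpolated tracking function exists, but its call in the event graph is disconnected.
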(event EventBeginPlay
  (bind _self self)
  (Utilities|FlowControl|Sequence
    (:then_0
      ;[1 1 1] Chequea si existe el BP_CameraManager en la escena
      (bind _returnvalue (Actor|GetActorOfClass "/Game/Project_D/Blueprints/Cameras/BP_CameraManager.BP_CameraManager_C"))
      (Utilities|IsValid _returnvalue
        (:Is%20Valid
          (Variables|Default|SetCameraManagerRef _returnvalue))
        (:Is%20Not%20Valid
          (Development|PrintString "CameraManagerNotFound"))))
    (:then_1
      (if (Variables|Default|GetIsLevelStartCamera)
        (Game|Player|SetViewTargetwithBlend (Game|GetPlayerController 0) _self 0.0 "VTBlend_Linear" 0.0 false)
        (Default|SetActiveCamera (Variables|Default|GetCameraManagerRef) _self)
        (CallFunction|SnaptoCharacterView)))))

(event EventTick
  (params (DeltaSeconds :type Float%20%28single-precision%29))
  (Variables|Default|SetDelta%20Seconds DeltaSeconds)
  (if (not (== (Variables|/Game/Project_D/Blueprints/Cameras/BP_CameraManager.BP_CameraManager_C|GetCurrentActiveCamera (Variables|Default|GetCameraManagerRef)) self))
    (Components|Tick|SetComponentTickEnabled (Variables|Default|GetCamera) false)))

(fn ConstructionScript)

(fn SnaptoCharacterView
  (if (Variables|Default|GetIsTrackingCamera)
    (Transformation|SetWorldRotation (Variables|Default|GetRoot) (Math|Rotator|FindLookatRotation (Transformation|GetWorldLocation (Variables|Default|GetRoot)) (Transformation|GetActorLocation (Game|GetPlayerCharacter 0))) false false)))

(fn TrackingCamera
  (Variables|Default|SetCurrentRotation (Transformation|GetWorldRotation (Variables|Default|GetCamera)))
  (Transformation|SetWorldRotation (Variables|Default|GetCamera) (Math|Interpolation|RInterpTo (Variables|Default|GetCurrentRotation) (Math|Rotator|FindLookatRotation (Transformation|GetWorldLocation (Variables|Default|GetCamera)) (Transformation|GetActorLocation (Game|GetPlayerCharacter 0))) (Variables|Default|GetDelta%20Seconds) (Variables|Default|GetInterp%20Speed)) false false))